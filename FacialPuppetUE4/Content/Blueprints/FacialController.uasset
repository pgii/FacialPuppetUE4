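; FacialController drives facial morph targets on a referenced skeletal mesh from values tagged with gamepad key enums.
; FacialDataReceive looks up the key in GamepadMorphMap to get a morph name and inverse flag, skipping unmapped keys through a "None" fallback.
; SetFacialMorph applies the value to that morph target, negating it when the mapping is flagged as inverse.
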(event Custom|FacialDataReceive
  (params (GamepadKeysEnum :type GamepadKeysEnum%20Enum :default "NewEnumerator0") (Value :type Float%20%28single-precision%29))
  (bind _facialmorphstruct (CallFunction|GetFacialMorphStruct GamepadKeysEnum))
  (if (Utilities|Name|NotEqual(Name) (.MorphName (Utilities|Struct|BreakFacialMorphStruct _facialmorphstruct)) "None")
    (CallFunction|SetFacialMorph Value _facialmorphstruct)))

(event Custom|SetFacialMorph
  (params (value :type Float%20%28single-precision%29) (FacialMorphStruct :type Facial%20Morph%20Struct%20Structure))
  (bind (_morphname _inverse) (Utilities|Struct|BreakFacialMorphStruct FacialMorphStruct))
  (Components|SkeletalMesh|SetMorphTarget (Variables|/Script/Engine.SkeletalMeshActor|GetSkeletalMeshComponent (Variables|Default|GetSkeletalMesh)) _morphname (Math|Float|SelectFloat (* value -1.0) value _inverse) true))

(fn ConstructionScript)

(fn GetFacialMorphStruct
  (params (GamepadKeysEnum :type GamepadKeysEnum%20Enum :default "NewEnumerator0"))
  (bind _gamepadmorphmap (Variables|Default|GetGamepadMorphMap))
  (bind (_value _returnvalue) (Utilities|Map|Find _gamepadmorphmap GamepadKeysEnum))
  (if _returnvalue
    (return _value)
    (else
      (return (Utilities|Struct|MakeFacialMorphStruct "None" false)))))