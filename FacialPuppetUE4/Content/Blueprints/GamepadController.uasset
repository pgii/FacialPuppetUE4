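; Gamepad input actor that drives a facial animation rig by forwarding controller input as enum-keyed values to a FacialController.
; On BeginPlay it enables input, finds the first FacialController in the level and creates the GUIWidget_BP overlay.
; Each input goes to both the controller and the widget through FacialDataReceive.
; Stick axes split into per-direction keys by sign, triggers pass analog values, shoulders act while held, and face buttons toggle on and off.
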(event EventBeginPlay
  ;[1 1 1] Begin play
  (Input|EnableInput (Game|GetPlayerController 0))
  (bind _outactors (Actor|GetAllActorsOfClass "/Game/Blueprints/FacialController.FacialController_C"))
  (Variables|Default|SetFacialController (Utilities|Array|Get(acopy) _outactors))
  (bind _returnvalue (UserInterface|CreateWidget "/Game/Blueprints/GUIWidget_BP.GUIWidget_BP_C"))
  (bind _output_get (Variables|Default|SetGUIWidget _returnvalue))
  (UserInterface|Viewport|AddtoViewport _output_get 0))

(event Input|GamepadEvents|GamepadLeftY
  (params (AxisValue :type Float%20%28single-precision%29))
  (bind _guiwidget (Variables|Default|GetGUIWidget))
  (bind _facialcontroller (Variables|Default|GetFacialController))
  ;[1 1 1] Left Stick
  (if (> AxisValue 0.0)
    (Default|FacialDataReceive _facialcontroller "NewEnumerator1" AxisValue)
    (Utilities|IsValid _guiwidget
      (:Is%20Valid
        (Default|FacialDataReceive _guiwidget "NewEnumerator1" AxisValue)))
    (else
      (Default|FacialDataReceive _facialcontroller "NewEnumerator2" AxisValue)
      (Utilities|IsValid _guiwidget
        (:Is%20Valid
          (Default|FacialDataReceive _guiwidget "NewEnumerator2" AxisValue))))))

(event Input|GamepadEvents|GamepadRightX
  (params (AxisValue :type Float%20%28single-precision%29))
  (bind _facialcontroller (Variables|Default|GetFacialController))
  (bind _guiwidget (Variables|Default|GetGUIWidget))
  ;[1 1 1] Right Stick
  (if (> AxisValue 0.0)
    (Default|FacialDataReceive _facialcontroller "NewEnumerator7" AxisValue)
    (Utilities|IsValid _guiwidget
      (:Is%20Valid
        (Default|FacialDataReceive _guiwidget "NewEnumerator7" AxisValue)))
    (else
      (Default|FacialDataReceive _facialcontroller "NewEnumerator8" AxisValue)
      (Utilities|IsValid _guiwidget
        (:Is%20Valid
          (Default|FacialDataReceive _guiwidget "NewEnumerator8" AxisValue))))))

(event Input|GamepadEvents|GamepadLeftX
  (params (AxisValue :type Float%20%28single-precision%29))
  (bind _guiwidget (Variables|Default|GetGUIWidget))
  (bind _facialcontroller (Variables|Default|GetFacialController))
  ;[1 1 1] Left Stick
  (if (> AxisValue 0.0)
    (Default|FacialDataReceive _facialcontroller "NewEnumerator4" AxisValue)
    (Utilities|IsValid _guiwidget
      (:Is%20Valid
        (Default|FacialDataReceive _guiwidget "NewEnumerator4" AxisValue)))
    (else
      (Default|FacialDataReceive _facialcontroller "NewEnumerator3" AxisValue)
      (Utilities|IsValid _guiwidget
        (:Is%20Valid
          (Default|FacialDataReceive _guiwidget "NewEnumerator3" AxisValue))))))

(event Input|GamepadEvents|GamepadRightY
  (params (AxisValue :type Float%20%28single-precision%29))
  (bind _facialcontroller (Variables|Default|GetFacialController))
  (bind _guiwidget (Variables|Default|GetGUIWidget))
  ;[1 1 1] Right Stick
  (if (> AxisValue 0.0)
    (Default|FacialDataReceive _facialcontroller "NewEnumerator5" AxisValue)
    (Utilities|IsValid _guiwidget
      (:Is%20Valid
        (Default|FacialDataReceive _guiwidget "NewEnumerator5" AxisValue)))
    (else
      (Default|FacialDataReceive _facialcontroller "NewEnumerator6" AxisValue)
      (Utilities|IsValid _guiwidget
        (:Is%20Valid
          (Default|FacialDataReceive _guiwidget "NewEnumerator6" AxisValue))))))

(event Input|GamepadEvents|GamepadLeftTriggerAxis
  (params (AxisValue :type Float%20%28single-precision%29))
  (bind _guiwidget (Variables|Default|GetGUIWidget))
  ;[1 1 1] Left Trigger
  (Default|FacialDataReceive (Variables|Default|GetFacialController) "NewEnumerator12" AxisValue)
  (Utilities|IsValid _guiwidget
    (:Is%20Valid
      (Default|FacialDataReceive _guiwidget "NewEnumerator12" AxisValue))))

(event Input|GamepadEvents|GamepadRightTriggerAxis
  (params (AxisValue :type Float%20%28single-precision%29))
  (bind _guiwidget (Variables|Default|GetGUIWidget))
  ;[1 1 1] Left Trigger
  (Default|FacialDataReceive (Variables|Default|GetFacialController) "NewEnumerator13" AxisValue)
  (Utilities|IsValid _guiwidget
    (:Is%20Valid
      (Default|FacialDataReceive _guiwidget "NewEnumerator13" AxisValue))))

(event Input|GamepadEvents|GamepadFaceButtonRight
  (params (Key :type Key%20Structure))
  (bind _guiwidget (Variables|Default|GetGUIWidget))
  ;[1 1 1] Face Button
  (:Pressed
    (bind _output_get (Variables|Default|SetFaceButtonRightEnabled (not (Variables|Default|GetFaceButtonRightEnabled))))
    (Default|FacialDataReceive (Variables|Default|GetFacialController) "NewEnumerator21" (Math|Float|SelectFloat 1.0 0.0 _output_get))
    (Utilities|IsValid _guiwidget
      (:Is%20Valid
        (Default|FacialDataReceive _guiwidget "NewEnumerator21" (Math|Float|SelectFloat 1.0 0.0 _output_get))))))

(event Input|GamepadEvents|GamepadLeftShoulder
  (params (Key :type Key%20Structure))
  (bind _guiwidget (Variables|Default|GetGUIWidget))
  (bind _facialcontroller (Variables|Default|GetFacialController))
  ;[1 1 1] Left Shoulder
  (:Pressed
    (Default|FacialDataReceive _facialcontroller "NewEnumerator10" 1.0)
    (Utilities|IsValid _guiwidget
      (:Is%20Valid
        (Default|FacialDataReceive _guiwidget "NewEnumerator10" 1.0))))
  (:Released
    (Default|FacialDataReceive _facialcontroller "NewEnumerator10" 0.0)
    (Utilities|IsValid _guiwidget
      (:Is%20Valid
        (Default|FacialDataReceive _guiwidget "NewEnumerator10" 0.0)))))

(event Input|GamepadEvents|GamepadRightShoulder
  (params (Key :type Key%20Structure))
  (bind _guiwidget (Variables|Default|GetGUIWidget))
  (bind _facialcontroller (Variables|Default|GetFacialController))
  ;[1 1 1] Left Shoulder
  (:Pressed
    (Default|FacialDataReceive _facialcontroller "NewEnumerator11" 1.0)
    (Utilities|IsValid _guiwidget
      (:Is%20Valid
        (Default|FacialDataReceive _guiwidget "NewEnumerator11" 1.0))))
  (:Released
    (Default|FacialDataReceive _facialcontroller "NewEnumerator11" 0.0)
    (Utilities|IsValid _guiwidget
      (:Is%20Valid
        (Default|FacialDataReceive _guiwidget "NewEnumerator11" 0.0)))))

(event Input|GamepadEvents|GamepadFaceButtonTop
  (params (Key :type Key%20Structure))
  (bind _guiwidget (Variables|Default|GetGUIWidget))
  ;[1 1 1] Face Button
  (:Pressed
    (bind _output_get (Variables|Default|SetFaceButtonTopEnabled (not (Variables|Default|GetFaceButtonTopEnabled))))
    (Default|FacialDataReceive (Variables|Default|GetFacialController) "NewEnumerator18" (Math|Float|SelectFloat 1.0 0.0 _output_get))
    (Utilities|IsValid _guiwidget
      (:Is%20Valid
        (Default|FacialDataReceive _guiwidget "NewEnumerator18" (Math|Float|SelectFloat 1.0 0.0 _output_get))))))

(event Input|GamepadEvents|GamepadFaceButtonBottom
  (params (Key :type Key%20Structure))
  (bind _guiwidget (Variables|Default|GetGUIWidget))
  ;[1 1 1] Face Button
  (:Pressed
    (bind _output_get (Variables|Default|SetFaceButtonBottomEnabled (not (Variables|Default|GetFaceButtonBottomEnabled))))
    (Default|FacialDataReceive (Variables|Default|GetFacialController) "NewEnumerator19" (Math|Float|SelectFloat 1.0 0.0 _output_get))
    (Utilities|IsValid _guiwidget
      (:Is%20Valid
        (Default|FacialDataReceive _guiwidget "NewEnumerator19" (Math|Float|SelectFloat 1.0 0.0 _output_get))))))

(event Input|GamepadEvents|GamepadFaceButtonLeft
  (params (Key :type Key%20Structure))
  (bind _guiwidget (Variables|Default|GetGUIWidget))
  ;[1 1 1] Face Button
  (:Pressed
    (bind _output_get (Variables|Default|SetFaceButtonLeftEnabled (not (Variables|Default|GetFaceButtonLeftEnabled))))
    (Default|FacialDataReceive (Variables|Default|GetFacialController) "NewEnumerator20" (Math|Float|SelectFloat 1.0 0.0 _output_get))
    (Utilities|IsValid _guiwidget
      (:Is%20Valid
        (Default|FacialDataReceive _guiwidget "NewEnumerator20" (Math|Float|SelectFloat 1.0 0.0 _output_get))))))

(fn ConstructionScript)